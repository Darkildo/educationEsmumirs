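; BP_generatedTile is a self-replicating floor tile for endless level generation.
; When a player-controlled pawn overlaps R, it spawns another copy one tile length along world -X.
; On BeginPlay it spawns a Cube_random_spawn at one of three child-actor target points, picked randomly, and slightly raises the player's clamped walk speed.
; Tick destroys the tile once the player pawn is far away.
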(event OnComponentBeginOverlap(r)
  (params (OverlappedComponent :type Primitive%20Component%20Object%20Reference) (OtherActor :type Actor%20Object%20Reference) (OtherComp :type Primitive%20Component%20Object%20Reference) (OtherBodyIndex :type Integer) (bFromSweep :type Boolean) (SweepResult :type Hit%20Result%20Structure%20%28by%20ref%29))
  (bind _aspawn (Utilities|Casting|CastToPawn OtherActor))
  (if (Pawn|IsPlayerControlled _aspawn)
    (CallFunction|GenerateNewFloor)))

(event Custom|Generate%20new%20floor
  (bind _defaultsceneroot (Variables|Default|GetDefaultSceneRoot))
  (bind _returnvalue (Transformation|GetWorldTransform _defaultsceneroot))
  (bind (_x _y _z) (Math|Vector|BreakVector (.location _returnvalue)))
  ;[0.3102 1 0.4051] определение дистанции и спаун последующего элемента
  (Game|SpawnActorfromClass "BP_generatedTile_C" (Math|Transform|MakeTransform (Math|Vector|MakeVector (- _x (* 2 (.X (Math|Vector|BreakVector (.BoxExtent (Collision|GetActorBounds false false)))))) _y _z) (.rotation _returnvalue) (.scale _returnvalue)) "Undefined" 0 0))

(event Custom|random%20spawn
  (bind _returnvalue (Math|Random|RandomIntegerinRange 0 2))
  (bind _array1 (Variables|Default|Getarray1))
  (bind _array1_2 (Variables|Default|Getarray1))
  (bind _output (Utilities|Array|Get(acopy) _array1_2 _returnvalue))
  (Utilities|Array|Add _array1 (Variables|/Script/Engine.ChildActorComponent|GetChildActor (Variables|Default|Gettarget%20point%201%20)))
  (Utilities|Array|Add _array1 (Variables|/Script/Engine.ChildActorComponent|GetChildActor (Variables|Default|Gettarget%20point%202)))
  (Utilities|Array|Add _array1 (Variables|/Script/Engine.ChildActorComponent|GetChildActor (Variables|Default|Gettarget%20point%203)))
  (if (Utilities|IsValid _output)
    (Game|SpawnActorfromClass "/Game/Bluerptins/cube_random_spawn.cube_random_spawn_C" (Transformation|GetActorTransform _output) "AlwaysSpawn" 0 0)
    (bind _asthird_person_character (Utilities|Casting|CastToThirdPersonCharacter (Game|GetPlayerCharacter 0)))
    (bind _output_get (Variables|/Script/Engine.CharacterMovementComponent|SetMaxWalkSpeed (Variables|/Script/Engine.Character|GetCharacterMovement _asthird_person_character) (Math|Float|Clamp(Float) (* (Variables|/Script/Engine.CharacterMovementComponent|GetMaxWalkSpeed (Variables|/Script/Engine.Character|GetCharacterMovement _asthird_person_character)) 1.01) 6e+02 2e+03)))
    (Development|PrintString (Utilities|String|ToString(Float) _output_get))
    (Utilities|FlowControl|Delay 1.5)))

(event EventBeginPlay
  (CallFunction|RandomSpawn))

(event EventTick
  (params (DeltaSeconds :type Float%20%28single-precision%29))
  (CallFunction|CheckConditionDestroy))

(fn ConstructionScript)

(fn CheckConditionDestroy
  (if (> (Transformation|GetDistanceTo (Game|Player|GetPlayerPawn 0) self) 2e+04)
    (Actor|DestroyActor)))